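; Revolver weapon Blueprint for the Sheriff character, with an early prototype of hitscan firing.
; Attach snaps the revolver to the weaponSocket on the player Sheriff's mesh.
; Fire line-traces forward from the Sheriff's follow camera on the Camera channel with debug drawing, then prints a placeholder message.
; The hit result is unused, and the event graph and construction script are empty.
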(fn `Attach`
  (bind _assheriff (cast `/Game/Blueprints/Sheriff` (`GameplayStatics.GetPlayerCharacter` 0)))
  (`self.K2_AttachToComponent` (`Character.Mesh` _assheriff) "weaponSocket" "SnapToTarget" "SnapToTarget" "SnapToTarget"))

(fn `Fire`
  (bind _returnvalue (`GameplayStatics.GetActorOfClass` "/Game/Blueprints/Sheriff.Sheriff_C"))
  (bind _followcamera (`/Game/Blueprints/Sheriff.FollowCamera` _returnvalue))
  (bind _returnvalue_2 (`SceneComponent.K2_GetComponentLocation` _followcamera))
  (`KismetSystemLibrary.LineTraceSingle` :`Start` _returnvalue_2 :`End` (+ _returnvalue_2 (* (`KismetMathLibrary.GetForwardVector` (`SceneComponent.K2_GetComponentRotation` _followcamera)) 3000.0)) :`TraceChannel` "TraceTypeQuery2" :`DrawDebugType` "ForDuration")
  (`KismetSystemLibrary.PrintString` "Hello"))

(fn `UserConstructionScript`)