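; Revolver weapon Blueprint that attaches to the Sheriff player's weapon socket and handles firing, ammo and reloading.
; Fire runs a debug-drawn line trace from the Sheriff's follow camera with random cone spread, spending a round and printing the count; the hit result is unused.
; Spent rounds accumulate in a refill counter, which Reload draws from the reserve ammo, printing a message when none remains.
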(event `self.ReceiveBeginPlay`
  ;[1 1 1] Begin Play
  (set `self.curAmmo` (`self.maxAmmo`)))

(event `Reload`
  (bind _totalammo (`self.totalAmmo`))
  ;[1 1 1] Reload
  (if (> _totalammo 0)
    (set `self.curAmmo` (+ (`KismetMathLibrary.Clamp` (`self.ammoToRefill`) 1 (`self.totalAmmo`)) (`self.curAmmo`)))
    (set `self.totalAmmo` (`KismetMathLibrary.Clamp` (- _totalammo (`self.ammoToRefill`)) 0 (`self.totalAmmo`)))
    (set `self.ammoToRefill` 0)
    (else
      (`KismetSystemLibrary.PrintString` "no more bullets"))))

(fn `Attach`
  (bind _assheriff (cast `/Game/Assets/Blueprints/Sheriff` (`GameplayStatics.GetPlayerCharacter` 0)))
  (`self.K2_AttachToComponent` (`Character.Mesh` _assheriff) "weaponSocket" "SnapToTarget" "SnapToTarget" "SnapToTarget"))

(fn `BulletSpread`
  (params (muzzleDIr :type "Vector Structure") (maxAngle :type "Float (double-precision)"))
  (returns (shotRotation :type "Rotator Structure"))
  (return (`KismetMathLibrary.MakeRotFromX` (`KismetMathLibrary.RandomUnitVectorInConeInDegrees` muzzleDIr maxAngle))))

(fn `Fire`
  (if (> (`self.curAmmo`) 0)
    (bind _returnvalue (`GameplayStatics.GetActorOfClass` "/Game/Assets/Blueprints/Sheriff.Sheriff_C"))
    (bind _followcamera (`/Game/Assets/Blueprints/Sheriff.FollowCamera` _returnvalue))
    (bind _returnvalue_2 (`SceneComponent.K2_GetComponentLocation` _followcamera))
    (`KismetSystemLibrary.LineTraceSingle` :`Start` _returnvalue_2 :`End` (+ _returnvalue_2 (* (`self.BulletSpread` (`KismetMathLibrary.GetForwardVector` (`SceneComponent.K2_GetComponentRotation` _followcamera)) (`self.bulletCone`)) 3000.0)) :`TraceChannel` "TraceTypeQuery2" :`DrawDebugType` "ForDuration" :`DrawTime` 0.5)
    (bind _result (`/Engine/EditorBlueprintResources/StandardMacros.DecrementInt` (`self.curAmmo`))
      (:`  `
        (`/Engine/EditorBlueprintResources/StandardMacros.IncrementInt` (`self.ammoToRefill`)
          (:`  `
            (`KismetSystemLibrary.PrintString` (`KismetStringLibrary.Conv_IntToString` (`KismetMathLibrary.Clamp` _result 0 6)))))))))

(fn `UserConstructionScript`)