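; TrainingAreaTrigger is a box trigger that moves the Sheriff between the BaseMap and TrainingArea levels.
; On overlap it checks the current level name, disables player input, shows a Fade widget and opens the other level after a short delay.
; When returning to BaseMap, it also stores the spawn location and a FromTraining flag on the SheriffShenanigans game instance, just after the OpenLevel call.
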(event `self.Box.OnComponentBeginOverlap`
  (params (OverlappedComponent :type "PrimitiveComponent Object Reference") (OtherActor :type "Actor Object Reference") (OtherComp :type "PrimitiveComponent Object Reference") (OtherBodyIndex :type Integer) (bFromSweep :type Boolean) (SweepResult :type "HitResult Structure (by ref)"))
  (if (== (`GameplayStatics.GetObjectClass` OtherActor) "/Game/Assets/Blueprints/Sheriff.Sheriff_C")
    (bind _returnvalue (`GameplayStatics.GetCurrentLevelName` true))
    (if (== _returnvalue "BaseMap")
      (`self.DisableInput` (`GameplayStatics.GetPlayerCharacter` 0) null)
      (bind _returnvalue_2 (`|CreateWidget` "/Game/Assets/UI/Fade.Fade_C"))
      (`UserWidget.AddToViewport` _returnvalue_2 0)
      (`KismetSystemLibrary.Delay` 2.0)
      (`GameplayStatics.OpenLevelBySoftObjectPtr` "/Game/Assets/Maps/TrainingArea.TrainingArea")
      (else
        (`self.DisableInput` (`GameplayStatics.GetPlayerCharacter` 0) null)
        (bind _returnvalue_3 (`|CreateWidget` "/Game/Assets/UI/Fade.Fade_C"))
        (`UserWidget.AddToViewport` _returnvalue_3 0)
        (`KismetSystemLibrary.Delay` 2.0)
        (`GameplayStatics.OpenLevelBySoftObjectPtr` "/Game/Assets/Maps/BaseMap.BaseMap")
        (bind _assheriff_shenanigans_instance (cast `/Game/Assets/Blueprints/SheriffShenanigans_Instance` (`GameplayStatics.GetGameInstance`)))
        (set `/Game/Assets/Blueprints/SheriffShenanigans_Instance.playerSpawnLocT` (`self.baseMapSpawnLoc`) _assheriff_shenanigans_instance)
        (set `/Game/Assets/Blueprints/SheriffShenanigans_Instance.fromTraining` true _assheriff_shenanigans_instance)))))

(fn `UserConstructionScript`)